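; BP_AGILA_Pawn is a physics-driven AGILA pawn with a health bar HUD and speed-based effects.
; BeginPlay adds the HUD widget to the viewport and copies MouseSens into MouseSensitivity.
; Tick computes mesh speed from physics velocity, prints it for debugging, and shows the left and right Niagara effects only while it exceeds SpeedVar.
; Hit events set a DidHit flag, with no movement or damage logic in these graphs.
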(event `self.ReceiveBeginPlay`
  (bind _returnvalue (`|CreateWidget` "/Game/HealthUI/HealthBarHud.HealthBarHud_C" (`GameplayStatics.GetPlayerController` 0)))
  (`UserWidget.AddToViewport` _returnvalue 0)
  (set `self.mouseSensitivity` (`self.Mouse Sens`)))

(event `self.ReceiveTick`
  (params (DeltaSeconds :type "Float (single-precision)"))
  (bind _returnvalue (`PrimitiveComponent.GetPhysicsLinearVelocity` (`self.mesh`) "None"))
  (bind _returnvalue_2 (`KismetMathLibrary.Sqrt` (+ (`KismetMathLibrary.Square` (.x _returnvalue)) (`KismetMathLibrary.Square` (.y _returnvalue)) (`KismetMathLibrary.Square` (.z _returnvalue)))))
  (bind _output_get (set `self.speed` _returnvalue_2))
  (`KismetSystemLibrary.PrintString` (`KismetStringLibrary.Conv_DoubleToString` _output_get))
  (if (> _returnvalue_2 (`self.SpeedVar`))
    (`SceneComponent.SetVisibility` (`self.Niagara_Left`) true false)
    (`SceneComponent.SetVisibility` (`self.Niagara_Right`) true false)
    (else
      (`SceneComponent.SetVisibility` (`self.Niagara_Left`) false false)
      (`SceneComponent.SetVisibility` (`self.Niagara_Right`) false false))))

(event `self.ReceiveActorBeginOverlap`
  (params (OtherActor :type "Actor Object Reference")))

(event `self.ReceiveHit`
  (params (MyComp :type "PrimitiveComponent Object Reference") (Other :type "Actor Object Reference") (OtherComp :type "PrimitiveComponent Object Reference") (bSelfMoved :type Boolean) (HitLocation :type "Vector Structure") (HitNormal :type "Vector Structure") (NormalImpulse :type "Vector Structure") (Hit :type "HitResult Structure (by ref)"))
  (set `self.didHit` true))

(fn `UserConstructionScript`)