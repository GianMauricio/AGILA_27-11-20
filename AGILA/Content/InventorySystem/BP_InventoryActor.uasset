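; BP_InventoryActor is an actor that owns an Inventory and lets the player toggle it with the Inventory input, enabled for player controller 0 on BeginPlay.
; Its Notify event wraps ObjectToAdd in a zero-quantity slot structure, passes it to AddToInventory and prints debug success or failure text.
; SendStruct and ToggleAddInventory are empty stubs, the latter holding only disconnected leftover add logic.
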(event `InputAction|Inventory`
  (params (Key :type "Key Structure"))
  (:`Pressed`
    (`/Game/InventorySystem/InventoryComponent.ToggleInventory` (`self.Inventory`))))

(event `self.ReceiveBeginPlay`
  (`self.EnableInput` (`GameplayStatics.GetPlayerController` 0)))

(event `self.ReceiveTick`
  (params (DeltaSeconds :type "Float (single-precision)")))

(event `/Game/InventorySystem/ItemInterface.Notify`
  (`KismetSystemLibrary.PrintString` "Got Notification")
  (`/Game/InventorySystem/ItemInterface.SendStruct` (struct))
  (`KismetSystemLibrary.PrintString` "Recieved Info")
  (bind _success (`/Game/InventorySystem/InventoryComponent.AddToInventory` (`self.Inventory`) (make `/Game/InventorySystem/SlotStructure` (`self.ObjectToAdd`))))
  (if _success
    (`KismetSystemLibrary.PrintString` "SUCCESS BIH")
    (else
      (`KismetSystemLibrary.PrintString` "wtf u doin bih"))))

(fn `SendStruct`
  (params (itemStruct :type "/Game/InventorySystem/ItemStructure Structure"))
  (returns (itemReturn :type "/Game/InventorySystem/ItemStructure Structure"))
  (return))

(fn `ToggleAddInventory`)

(fn `UserConstructionScript`)